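; BP_MentalAttributes is a sphere actor acting as either an Intellect/Spirit attribute source or, with IsMechanism set, a mechanism triggered by that attribute.
; On overlap, a source gives an attribute-less BP_Character its attribute and shows the matching material.
; A mechanism fires once for a character holding a differing attribute, clearing it and calling OnPlay, which only prints a string here.
; The construction script colors the sphere by attribute.
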(event OnComponentBeginOverlap(SphereCollision)
  (params (OverlappedComponent :type Primitive%20Component%20Object%20Reference) (OtherActor :type Actor%20Object%20Reference) (OtherComp :type Primitive%20Component%20Object%20Reference) (OtherBodyIndex :type Integer) (bFromSweep :type Boolean) (SweepResult :type Hit%20Result%20Structure%20%28by%20ref%29))
  (bind _asbp_character (Utilities|Casting|CastToBP_Character OtherActor))
  (switch Utilities|FlowControl|Switch|SwitchonE_MentalAttributes (Variables|/Game/BluePoch/BluePrint/Character/BP_Character.BP_Character_C|GetMentalAttributes _asbp_character)
    (:NewEnumerator2
      (if (not (Variables|Default|GetIsMechanism))
        (Variables|/Game/BluePoch/BluePrint/Character/BP_Character.BP_Character_C|SetMentalAttributes _asbp_character (Variables|Default|GetMentalAttributes))
        (Rendering|SetVisibility (Variables|/Game/BluePoch/BluePrint/Character/BP_Character.BP_Character_C|GetMentalAttribute _asbp_character) true false)
        (switch Utilities|FlowControl|Switch|SwitchonE_MentalAttributes (Variables|Default|GetMentalAttributes)
          (:NewEnumerator0
            (Rendering|Material|SetMaterial (Variables|/Game/BluePoch/BluePrint/Character/BP_Character.BP_Character_C|GetMentalAttribute _asbp_character) 0 "/Game/BluePoch/BluePrint/MentalAttributes/Material/M_Intellect.M_Intellect"))
          (:NewEnumerator1
            (Rendering|Material|SetMaterial (Variables|/Game/BluePoch/BluePrint/Character/BP_Character.BP_Character_C|GetMentalAttribute _asbp_character) 0 "/Game/BluePoch/BluePrint/MentalAttributes/Material/M_Spirit.M_Spirit")))))
    (:NewEnumerator0
      (if (Math|Boolean|ANDBoolean (Variables|Default|GetIsMechanism) (not (Utilities|Enum|Equal(Enum) (Variables|/Game/BluePoch/BluePrint/Character/BP_Character.BP_Character_C|GetMentalAttributes _asbp_character) (Variables|Default|GetMentalAttributes))) (not (Variables|Default|GetIsUsed))) :!label _label
        (Rendering|SetVisibility (Variables|/Game/BluePoch/BluePrint/Character/BP_Character.BP_Character_C|GetMentalAttribute _asbp_character) false false)
        (Variables|/Game/BluePoch/BluePrint/Character/BP_Character.BP_Character_C|SetMentalAttributes _asbp_character "NewEnumerator2")
        (CallFunction|OnPlay)
        (Variables|Default|SetIsUsed true)))
    (:NewEnumerator1
      (goto _label))))

(event Custom|OnPlay
  (Development|PrintString "咪"))

(event EventBeginPlay)

(event Collision|EventActorBeginOverlap
  (params (OtherActor :type Actor%20Object%20Reference)))

(event EventTick
  (params (DeltaSeconds :type Float%20%28single-precision%29)))

(fn ConstructionScript
  (bind _sphere (Variables|Default|GetSphere))
  (switch Utilities|FlowControl|Switch|SwitchonE_MentalAttributes (Variables|Default|GetMentalAttributes)
    (:NewEnumerator0
      (Rendering|Material|SetMaterial _sphere 0 "/Game/BluePoch/BluePrint/MentalAttributes/Material/M_Intellect.M_Intellect"))
    (:NewEnumerator1
      (Rendering|Material|SetMaterial _sphere 0 "/Game/BluePoch/BluePrint/MentalAttributes/Material/M_Spirit.M_Spirit"))))