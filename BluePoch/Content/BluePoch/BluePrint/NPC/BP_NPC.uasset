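; BP_NPC is an NPC that trades the player's coins for a feather.
; When a BP_Character overlaps its Box, it picks a price that rises with the character's current JumpMaxCount.
; If the character has enough Coins, it deducts the price and spawns a BP_Feather at Arrow1's transform.
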(event OnComponentBeginOverlap(Box)
  (params (OverlappedComponent :type Primitive%20Component%20Object%20Reference) (OtherActor :type Actor%20Object%20Reference) (OtherComp :type Primitive%20Component%20Object%20Reference) (OtherBodyIndex :type Integer) (bFromSweep :type Boolean) (SweepResult :type Hit%20Result%20Structure%20%28by%20ref%29))
  (bind _asbp_character (Utilities|Casting|CastToBP_Character OtherActor))
  (if (>= (Variables|/Game/BluePoch/BluePrint/Character/BP_Character.BP_Character_C|GetCoins _asbp_character) (Utilities|Select :Index (Variables|/Script/Engine.Character|GetJumpMaxCount _asbp_character) :Option%200 5 :Option%201 10 :Option%202 30 :Option%203 40))
    (Variables|/Game/BluePoch/BluePrint/Character/BP_Character.BP_Character_C|SetCoins _asbp_character (- (Variables|/Game/BluePoch/BluePrint/Character/BP_Character.BP_Character_C|GetCoins _asbp_character) (Utilities|Select :Index (Variables|/Script/Engine.Character|GetJumpMaxCount _asbp_character) :Option%200 5 :Option%201 10 :Option%202 30 :Option%203 40)))
    (Game|SpawnActorfromClass "/Game/BluePoch/BluePrint/Feather/BP_Feather.BP_Feather_C" (Transformation|GetWorldTransform (Variables|Default|GetArrow1)) "Undefined" "MultiplyWithRoot" 0 0)))

(event EventBeginPlay)

(event Collision|EventActorBeginOverlap
  (params (OtherActor :type Actor%20Object%20Reference)))

(event EventTick
  (params (DeltaSeconds :type Float%20%28single-precision%29)))

(fn ConstructionScript)