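; BP_Possess is a possessable actor that hands player control back to the character stored in the GI_Blue game instance.
; SwitchCharacter checks that stored character is valid, then has the first player controller unpossess its current pawn and possess it.
; The character is then moved to this actor's location, offset backward along world X.
; Construction runs the parent script and clears the IsCharacter flag.
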(event EventSwitchCharacter
  (bind _returnvalue (Transformation|GetActorLocation))
  (bind _asgi_blue (Utilities|Casting|CastToGI_Blue (Game|GetGameInstance)))
  (Utilities|IsValid (Variables|/Game/BluePoch/GamePlay/GI_Blue.GI_Blue_C|GetCharacter _asgi_blue)
    (:Is%20Valid
      (Pawn|UnPossess (Game|GetPlayerController 0))
      (Pawn|Possess (Game|GetPlayerController 0) (Variables|/Game/BluePoch/GamePlay/GI_Blue.GI_Blue_C|GetCharacter _asgi_blue))
      (Transformation|SetActorLocation (Variables|/Game/BluePoch/GamePlay/GI_Blue.GI_Blue_C|GetCharacter _asgi_blue) (Math|Vector|MakeVector (+ (.x _returnvalue) -1e+02) (.y _returnvalue) (.z _returnvalue)) false false))))

(fn ConstructionScript
  (|CallParentFunction)
  (Variables|Default|SetIsCharacter false))